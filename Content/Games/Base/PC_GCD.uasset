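; PC_GCD player controller that sets up the HUD and spawns the player's pawn, either a saved character or a god-mode spectator.
; BeginPlay builds the main and shortcut bars, then reads the SelectSaveFile slot, falling back to BP_GodSpectator with cursor input when no valid class is saved.
; Spawning is authority-gated, using a random PlayerStart before possession.
; It also toggles the ESC menu via FlipFlop and offers a cursor-to-ground trace helper.
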(event Custom|生成控制角色
  (params (玩家控制器 :type Player%20Controller%20Object%20Reference) (类型 :type Actor%20Class%20Reference))
  ;[1 1 1] 服务器：非上帝生成
  (Networking|SwitchHasAuthority
    (:Authority
      (if (Utilities|IsValidClass 类型)
        (CallFunction|从玩家起始点生成指定Actor 玩家控制器 类型)))))

(event Custom|打开ESC菜单
  ;[1 1 1] 打开ESC菜单
  (Utilities|FlowControl|FlipFlop
    (:A
      (bind _returnvalue (UserInterface|CreateWidget "/Game/Games/Base/W_EscMenu.W_EscMenu_C"))
      (UserInterface|Viewport|AddtoViewport _returnvalue 0))
    (:B
      (Widget|RemovefromParent _returnvalue)
      (Variables|Default|SetbShowMouseCursor false)
      (Input|SetInputModeGameOnly self))))

(event Custom|服务器：生成控制角色
  (params (玩家控制器 :type Player%20Controller%20Object%20Reference) (类型 :type Actor%20Class%20Reference))
  ;[1 1 1] 服务器：非上帝生成
  (if (Utilities|IsValidClass 类型)
    (CallFunction|从玩家起始点生成指定Actor 玩家控制器 类型)))

(event EventBeginPlay
  (bind _self self)
  (bind _self_2 self)
  ;[1 1 1] 初始化
  (bind _newparam (CallFunction|创建Bar主控件))
  (if _newparam
    (CallFunction|生成底部快捷栏Bar)
    (bind _returnvalue (SaveGame|LoadGamefromSlot "SelectSaveFile"))
    (bind _assg_select_actor (Utilities|Casting|CastToSG_SelectActor _returnvalue))
    (bind _output_get (Variables|Default|SetSelectSaveFile _assg_select_actor))
    (bind _output_get_2 (Variables|Default|Set是否是上帝模式 (not (Utilities|IsValidClass (Variables|/Game/Games/UI/SelectActor/SG_SelectActor.SG_SelectActor_C|GetActorClass _output_get)))))
    (if _output_get_2
      (CallFunction|生成控制角色 _self_2 "/Game/Games/Base/God/BP_GodSpectator.BP_GodSpectator_C")
      (Input|SetInputModeGameandUI _self 0 "DoNotLock" false)
      (Variables|Default|SetbShowMouseCursor _self true)
      (else
        (CallFunction|生成控制角色 _self_2 (Variables|/Game/Games/UI/SelectActor/SG_SelectActor.SG_SelectActor_C|GetActorClass _output_get))
        (Input|SetInputModeGameOnly self)))))

(event Input|ActionEvents|InputAction通用：打开菜单
  (params (Key :type Key%20Structure :default "None"))
  ;[1 1 1] 打开ESC菜单
  (:Pressed
    (CallFunction|打开ESC菜单)))

(fn ConstructionScript)

(fn 获得鼠标到地上位置
  (bind _hitresult (Game|Player|GetHitResultUnderCursorbyChannel "TraceTypeQuery1" true))
  (bind (_bblockinghit _binitialoverlap _time _distance _location _impactpoint _normal _impactnormal) (Collision|BreakHitResult _hitresult))
  (return _location (Math|Rotator|MakeRotationfromAxes _impactnormal "0, 0, 0" "0, 0, 0")))

(fn 从玩家起始点生成指定Actor
  (params (GCD玩家控制器 :type Player%20Controller%20Object%20Reference) (需要生成的Actor的类 :type Actor%20Class%20Reference))
  (bind _aspc_gcd (Utilities|Casting|CastToPC_GCD GCD玩家控制器))
  (Utilities|IsValid _aspc_gcd
    (:Is%20Valid
      (bind _outactors (Actor|GetAllActorsOfClass "/Script/Engine.PlayerStart"))
      (if (Utilities|IsValidClass 需要生成的Actor的类)
        (bind _returnvalue (Game|SpawnActorfromClass 需要生成的Actor的类 (Transformation|GetActorTransform (Utilities|Array|Get(acopy) _outactors (Math|Random|RandomIntegerinRange 0 (- (Utilities|Array|Length _outactors) 1)))) "AdjustIfPossibleButAlwaysSpawn" 0 0))
        (bind _aspawn (Utilities|Casting|CastToPawn _returnvalue))
        (Pawn|Possess _aspc_gcd _aspawn)))))

(fn 创建Bar主控件
  (bind _returnvalue (UserInterface|CreateWidget "/Game/Games/Base/Bar/W_BarMain.W_BarMain_C" self))
  (bind _output_get (Variables|Default|SetBar主控件 _returnvalue))
  (UserInterface|Viewport|AddtoViewport _output_get 0)
  (return true))

(fn 生成底部快捷栏Bar
  (bind _returnvalue (UserInterface|CreateWidget "/Game/Games/Base/Bar/ShortcutBar/W_ShortcutBar.W_ShortcutBar_C" (Game|GetPlayerController 0) 10))
  (bind _output_get (Variables|Default|Set底部快捷栏Bar控件 _returnvalue))
  (Widget|Panel|AddChild (Variables|/Game/Games/Base/Bar/W_BarMain.W_BarMain_C|Get底部Bar (Variables|Default|GetBar主控件)) _output_get))