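; God-mode spectator pawn giving RTS-style control of AI pieces (BP_AIBase) with a free-fly camera.
; An operation-mode state routes mouse input between box/click selection with foot markers, move or waypoint-route orders, and placement with a translucent preview respawned each tick.
; Server events spawn, destroy, move (AIMoveTo) and assign controllers, locking pieces to one player.
; BeginPlay builds the piece list UI and loads classes from a data table; HUD_God receives selection-box and route-line data.
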(event Custom|【线路】服务器：棋子沿着目标走
  (params (被移动的棋子 :type BP%20AI%20Base%20Object%20Reference) (目标 :type Actor%20Object%20Reference) (目标位置 :type Vector))
  ;[1 1 1] 【线路】服务器：棋子沿着目标走
  (if (== 目标 被移动的棋子)
    (AI|AIMoveTo 被移动的棋子 目标位置 0 5.0 false)
    (else
      (AI|AIMoveTo 被移动的棋子 "0, 0, 0" 目标 5.0 false))))

(event Custom|服务器：摧毁棋子
  (params (要摧毁的棋子 :type BP%20AI%20Base%20Object%20Reference))
  ;[1 1 1] 服务器：摧毁棋子
  (Actor|DestroyActor 要摧毁的棋子))

(event Custom|【单次】服务器：棋子移动到
  (params (被移动的棋子 :type Pawn%20Object%20Reference) (位置 :type Vector))
  ;[1 1 1] 【单次】服务器：命令棋子移动到指定位置
  (AI|AIMoveTo 被移动的棋子 位置 0 0.0 false))

(event Custom|服务器：给棋子设定目标
  (params (棋子 :type BP%20AI%20Base%20Object%20Reference) (目标 :type Array%20of%20Actor%20Object%20References) (目标位置 :type Array%20of%20Vectors) (棋子状态 :type Integer))
  ;[1 1 1] 服务器：给棋子设定控制者
)

(event Custom|服务器：给棋子设定控制者
  (params (棋子 :type BP%20AI%20Base%20Object%20Reference) (控制者 :type BP%20God%20Spectator%20Object%20Reference))
  ;[1 1 1] 服务器：给棋子设定控制者
  (Variables|/Game/Games/Base/AI/BP_AIBase.BP_AIBase_C|Set控制者 棋子 控制者))

(event Custom|服务器：生成棋子
  (params (Location :type Vector) (要生成的棋子类型 :type BP%20AI%20Base%20Class%20Reference))
  ;[1 1 1] 服务器：生成棋子
  (Game|SpawnActorfromClass 要生成的棋子类型 (Math|Transform|MakeTransform Location "0, 0, 0" "1,1,1") "AlwaysSpawn" 0 0))

(event Custom|生成AI棋子列表Bar
  (bind _returnvalue (Game|GetPlayerController 0))
  ;[1 1 1] 初始化：生成AI棋子列表Bar
  (bind _aspc_gcd (Utilities|Casting|CastToPC_GCD _returnvalue))
  (bind _returnvalue_2 (UserInterface|CreateWidget "/Game/Games/Base/Bar/AIBox/W_AIBox.W_AIBox_C" _returnvalue (Variables|/Game/Games/Base/PC_GCD.PC_GCD_C|GetBar主控件 _aspc_gcd) ""))
  (bind _output_get (Variables|Default|SetAI棋子Bar控件 _returnvalue_2))
  (Widget|Panel|AddChild (Variables|/Game/Games/Base/Bar/W_BarMain.W_BarMain_C|Get左侧Bar (Variables|/Game/Games/Base/PC_GCD.PC_GCD_C|GetBar主控件 _aspc_gcd)) _output_get))

(event EventBeginPlay
  (bind _ai数据表 (Variables|Default|GetAI数据表))
  ;[1 1 1] 初始化
  (Utilities|FlowControl|Sequence
    (:then_0
      (Networking|SwitchHasAuthority
        (:Authority
          (Class|Actor|AddActorWorldTransform (Math|Transform|MakeTransform "0,0.000000,1000.000000" "-45.000000, 0, 0" "1,1,1") true false))))
    (:then_1
      (bind _outrownames (DataTable|GetDataTableRowNames _ai数据表))
      (for _array_element _outrownames
        (bind _returnvalue (Utilities|GetDataTableRow _ai数据表 _array_element)
          (:then
            (Utilities|Array|Add (Variables|Default|Get可用的棋子类型) (.Class (Utilities|Struct|BreakS_AIPawn _returnvalue)))
            (Class|PlayerController|ClientSetHUD (Game|GetPlayerController 0) "/Game/Games/Base/God/HUD_God.HUD_God_C")))))
    (:then_2
      (bind _aspc_gcd (Utilities|Casting|CastToPC_GCD (Game|GetPlayerController 0)))
      (Variables|Default|SetBar主控件 (Variables|/Game/Games/Base/PC_GCD.PC_GCD_C|GetBar主控件 _aspc_gcd))
      (Variables|Default|Set底部快捷栏Bar控件 (Variables|/Game/Games/Base/PC_GCD.PC_GCD_C|Get底部快捷栏Bar控件 _aspc_gcd))
      (CallFunction|生成AI棋子列表Bar))))

(event Custom|同步指示标位置到棋子脚下
  (bind _被选中的棋子和脚底的指示标 (Variables|Default|Get被选中的棋子和脚底的指示标))
  ;[1 1 1] 【Tick】同步指示标位置到棋子脚下
  (bind _keys (Utilities|Map|Keys _被选中的棋子和脚底的指示标))
  (for _array_element _keys
    (Utilities|IsValid (.Value (Utilities|Map|Find _被选中的棋子和脚底的指示标 _array_element))
      (:Is%20Valid
        (Transformation|SetActorLocation (.Value (Utilities|Map|Find _被选中的棋子和脚底的指示标 _array_element)) (Transformation|GetWorldLocation (Variables|/Script/Engine.Character|GetMesh _array_element)) false false)))))

(event EventTick
  (params (DeltaSeconds :type Float%20%28single-precision%29))
  (bind _手中棋子的类型 (Variables|Default|Get手中棋子的类型))
  ;[1 1 1] Tick
  (Utilities|FlowControl|Sequence
    (:then_0
      (CallFunction|同步指示标位置到棋子脚下))
    (:then_2
      (Utilities|IsValid (Variables|Default|Get上次生成的未落下的棋子) :!label _label
        (:Is%20Valid
          (Actor|DestroyActor (Variables|Default|Get上次生成的未落下的棋子))
          (goto _label))
        (:Is%20Not%20Valid
          (if (Utilities|IsValidClass _手中棋子的类型)
            (bind _location (通用|获得鼠标在地面的位置))
            (bind _returnvalue (Game|SpawnActorfromClass _手中棋子的类型 (Math|Transform|MakeTransform (+ _location "0, 0,20.000000") "0, 0, 0" "1,1,1") "AdjustIfPossibleButDontSpawnIfColliding" 0 0))
            (Utilities|IsValid _returnvalue
              (:Is%20Valid
                (Rendering|Material|SetMaterial (Variables|/Script/Engine.Character|GetMesh _returnvalue) 0 "/Game/Games/Base/AI/Material/M_GreenTranslucence_Inst.M_GreenTranslucence_Inst")
                (Networking|SetReplicates _returnvalue false)
                (Variables|Default|Set上次生成的未落下的棋子 _returnvalue)))))))))

(event Input|ActionEvents|InputAction通用：数字快捷栏（顺序不能错）
  (params (Key :type Key%20Structure))
  ;[1 1 1] 数字键：使用快捷栏
  (:Pressed
    (bind _asw_bar_item_base (Utilities|Casting|CastToW_BarItemBase (Class|PanelWidget|GetChildat (Variables|/Game/Games/Base/Bar/Base/W_BarSlot.W_BarSlot_C|Get项目ItemBase (.Value (Utilities|Map|Find (Variables|/Game/Games/Base/Bar/ShortcutBar/W_ShortcutBar.W_ShortcutBar_C|Get按键-格子 (Variables|Default|Get底部快捷栏Bar控件)) Key))))))
    (Default|使用 _asw_bar_item_base)))

(event Input|ActionEvents|InputAction上帝模式：摧毁选中棋子
  (params (Key :type Key%20Structure))
  ;[1 1 1] 摧毁棋子
  (:Pressed
    (bind _keys (Utilities|Map|Keys (Variables|Default|Get被选中的棋子和脚底的指示标)))
    (for _array_element _keys
      (通用|摧毁棋子 _array_element))))

(event Input|ActionEvents|InputAction上帝模式：开始沿着导航路线走
  (params (Key :type Key%20Structure))
  ;[1 1 1] Ctrl+右键：给棋子设定目标路径
  (:Pressed
    (线路移动|【线路】棋子开始沿着之前设定的目标走)))

(event Input|ActionEvents|InputAction上帝模式：Ctrl+右键
  (params (Key :type Key%20Structure))
  ;[1 1 1] Ctrl+右键：给棋子设定目标路径
  (:Pressed
    (switch int (Variables|Default|Get当前操作模式)
      (:1
        (线路移动|【线路】给选中的棋子设定目标)))))

(event Input|ActionEvents|InputAction上帝模式：Ctrl+左键
  (params (Key :type Key%20Structure))
  (bind _被选中的棋子和脚底的指示标 (Variables|Default|Get被选中的棋子和脚底的指示标))
  ;[1 1 1] 按住Ctrl左键：多选场上的棋子
  (:Pressed
    (switch int (Variables|Default|Get当前操作模式)
      (:0
        (控制|清理上次选中的棋子的指示标))
      (:1
        _))
    (Variables|Default|Set当前操作模式 1)
    (bind _被点到的棋子 (控制|获得鼠标点击的棋子))
    (Utilities|IsValid _被点到的棋子
      (:Is%20Valid
        (Utilities|IsValid (.Value (Utilities|Map|Find _被选中的棋子和脚底的指示标 _被点到的棋子))
          (:Is%20Valid
            (Actor|DestroyActor (.Value (Utilities|Map|Find _被选中的棋子和脚底的指示标 _被点到的棋子)))
            (Utilities|Map|Remove _被选中的棋子和脚底的指示标 _被点到的棋子)
            (CallFunction|服务器：给棋子设定控制者 _被点到的棋子))
          (:Is%20Not%20Valid
            (bind _是否 (控制|判断棋子是否有控制者 _被点到的棋子))
            (if _是否
              (控制|选中棋子并在棋子底部生成指示标 _被点到的棋子))))))))

(event Input|ActionEvents|InputAction上帝模式：辅助控制
  (params (Key :type Key%20Structure))
  ;[1 1 1] 鼠标右键点击：开关可否转动屏幕/棋子移动/终止放棋
  (:Pressed
    (switch int (Variables|Default|Get当前操作模式)
      (:0
        (Variables|Default|Set是否可以转动屏幕 true))
      (:1
        (单次移动|【单次】让被选中的棋子立即执行一个目标))
      (:2
        (if (Utilities|IsValidClass (Variables|Default|Get手中棋子的类型))
          (Variables|Default|Set手中棋子的类型 0)
          (Variables|Default|Set当前操作模式 0)))))
  (:Released
    (Variables|Default|Set是否可以转动屏幕 false)))

(event Input|ActionEvents|InputAction上帝模式：主要控制
  (params (Key :type Key%20Structure))
  (bind _returnvalue (Game|GetPlayerController 0))
  (bind _上次生成的未落下的棋子 (Variables|Default|Get上次生成的未落下的棋子))
  (bind _手中棋子的类型 (Variables|Default|Get手中棋子的类型))
  (bind (_locationx _locationy) (Game|Player|GetMousePosition _returnvalue))
  (bind _returnvalue_2 (HUD|GetHUD _returnvalue))
  ;[1 1 1] 鼠标左键
  (:Pressed
    (switch int (Variables|Default|Get当前操作模式)
      (:0
        ;;[1 1 1] 鼠标左键：单选场上的棋子
        (bind _被点到的棋子 (控制|获得鼠标点击的棋子 :!label _label))
        (Utilities|IsValid _被点到的棋子
          (:Is%20Valid
            (bind _是否 (控制|判断棋子是否有控制者 _被点到的棋子))
            (if _是否
              (控制|清理上次选中的棋子的指示标)
              (控制|选中棋子并在棋子底部生成指示标 _被点到的棋子)
              (Variables|Default|Set当前操作模式 1)))
          (:Is%20Not%20Valid
            (Variables|Default|Set当前操作模式 0)
            ;;[1 1 1] 未单选到棋子触发框选
            (bind _ashud_god (Utilities|Casting|CastToHUD_God _returnvalue_2))
            (bind _output_get (Variables|/Game/Games/Base/God/HUD_God.HUD_God_C|Set是否触发框选 _ashud_god true))
            (Variables|Default|Set是否触发框选 _output_get)
            (bind _output_get_2 (Variables|/Game/Games/Base/God/HUD_God.HUD_God_C|SetBegin _ashud_god (Math|Vector2D|MakeVector2D _locationx _locationy)))
            (Variables|/Game/Games/Base/God/HUD_God.HUD_God_C|SetCurrent _ashud_god _output_get_2))))
      (:1
        (goto _label))
      (:2
        ;;[1 1 1] 鼠标左键：放置棋子
        (if (Utilities|IsValidClass _手中棋子的类型)
          (Utilities|IsValid _上次生成的未落下的棋子
            (:Is%20Valid
              (CallFunction|服务器：生成棋子 (Transformation|GetActorLocation _上次生成的未落下的棋子) _手中棋子的类型)
              (Actor|DestroyActor _上次生成的未落下的棋子)))))))
  (:Released
    (if (Variables|Default|Get是否触发框选)
      ;;[1 1 1] 框选结束
      (bind _ashud_god_2 (Utilities|Casting|CastToHUD_God _returnvalue_2))
      (bind _output_get_3 (Variables|/Game/Games/Base/God/HUD_God.HUD_God_C|Set是否触发框选 _ashud_god_2 false))
      (Variables|Default|Set是否触发框选 _output_get_3)
      (控制|清理上次选中的棋子的指示标)
      (for _array_element (Variables|Default|Get框选获得的棋子)
        (bind _asbp_aibase (Utilities|Casting|CastToBP_AIBase _array_element)
          (:then
            (bind _是否_2 (控制|判断棋子是否有控制者 _asbp_aibase))
            (if _是否_2
              (控制|选中棋子并在棋子底部生成指示标 _asbp_aibase)
              (Variables|Default|Set当前操作模式 1)))
          (:CastFailed
            (Variables|Default|Set当前操作模式 0)))))))

(event Input|ActionEvents|InputAction上帝模式：呼出棋子列表
  (params (Key :type Key%20Structure))
  ;[1 1 1] 打开棋子列表UI
  (:Pressed
    (Default|显示/隐藏Bar (Variables|Default|GetBar主控件) (Variables|Default|GetAI棋子Bar控件))))

(event Input|AxisEvents|InputAxis上帝模式：镜头远近
  (params (AxisValue :type Float%20%28single-precision%29))
  ;[1 1 1] 滚轮控制镜头远近
  (Class|Actor|AddActorWorldTransform (Math|Transform|MakeTransform (* (Math|Rotator|GetRotationXVector (Transformation|GetWorldRotation (Variables|/Script/Engine.Actor|GetRootComponent (Game|GetPlayerCameraManager 0)))) (* 100 AxisValue)) "0, 0, 0" "1,1,1") false false))

(event Input|AxisEvents|InputAxis通用：纵向移动
  (params (AxisValue :type Float%20%28single-precision%29))
  (bind _returnvalue (Pawn|GetControlRotation :!class /Script/Engine.Pawn))
  (bind _returnvalue_2 (Game|GetPlayerCameraManager 0))
  (bind _yaw (Math|Rotator|BreakRotator _returnvalue))
  (bind _rootcomponent (Variables|/Script/Engine.Actor|GetRootComponent _returnvalue_2))
  (bind _returnvalue_3 (Math|Rotator|MakeRotator 0.0 0.0 _yaw))
  (bind _returnvalue_4 (Transformation|GetWorldRotation _rootcomponent))
  ;[1 1 1] WASD控制
  (if (Variables|Default|Get是否可以转动屏幕)
    ;;[1 1 1] 右键按住时：前后移动
    (Pawn|Input|AddMovementInput (+ (* (Math|Rotator|GetRotationXVector _returnvalue_4) AxisValue) (* (Math|Vector|GetRightVector _returnvalue_4) (stale Input|AxisEvents|InputAxis通用：横向移动 AxisValue))) 1.0 false)
    (else
      ;;[1 1 1] 没有按住右键：平面移动
      (Pawn|Input|AddMovementInput (+ (* (Math|Vector|GetForwardVector _returnvalue_3) AxisValue) (* (Math|Vector|GetRightVector _returnvalue_3) (stale Input|AxisEvents|InputAxis通用：横向移动 AxisValue))) 1.0 false))))

(event Input|AxisEvents|InputAxis通用：横向移动
  (params (AxisValue :type Float%20%28single-precision%29))
  (bind _returnvalue (Pawn|GetControlRotation :!class /Script/Engine.Pawn))
  (bind _returnvalue_2 (Game|GetPlayerCameraManager 0))
  (bind _yaw (Math|Rotator|BreakRotator _returnvalue))
  (bind _rootcomponent (Variables|/Script/Engine.Actor|GetRootComponent _returnvalue_2))
  (bind _returnvalue_3 (Math|Rotator|MakeRotator 0.0 0.0 _yaw))
  (bind _returnvalue_4 (Transformation|GetWorldRotation _rootcomponent))
  ;[1 1 1] WASD控制
  (if (Variables|Default|Get是否可以转动屏幕)
    ;;[1 1 1] 右键按住时：前后移动
    (Pawn|Input|AddMovementInput (+ (* (Math|Rotator|GetRotationXVector _returnvalue_4) (stale Input|AxisEvents|InputAxis通用：纵向移动 AxisValue)) (* (Math|Vector|GetRightVector _returnvalue_4) AxisValue)) 1.0 false)
    (else
      ;;[1 1 1] 没有按住右键：平面移动
      (Pawn|Input|AddMovementInput (+ (* (Math|Vector|GetForwardVector _returnvalue_3) (stale Input|AxisEvents|InputAxis通用：纵向移动 AxisValue)) (* (Math|Vector|GetRightVector _returnvalue_3) AxisValue)) 1.0 false))))

(event Input|AxisEvents|InputAxis通用：上下看
  (params (AxisValue :type Float%20%28single-precision%29))
  (bind _returnvalue (Game|GetPlayerController 0))
  (bind (_locationx _locationy) (Game|Player|GetMousePosition _returnvalue))
  ;[1 1 1] 移动鼠标：【按住右键的同时移动鼠标】控制镜头旋转；【按住左键的同时移动鼠标】选择框
  (if (Variables|Default|Get是否触发框选)
    (bind _ashud_god (Utilities|Casting|CastToHUD_God (HUD|GetHUD _returnvalue)))
    (Variables|/Game/Games/Base/God/HUD_God.HUD_God_C|SetCurrent _ashud_god (Math|Vector2D|MakeVector2D _locationx _locationy))
    (elif (Variables|Default|Get是否可以转动屏幕)
      (Pawn|Input|AddControllerPitchInput AxisValue))))

(event Input|AxisEvents|InputAxis通用：左右看
  (params (AxisValue :type Float%20%28single-precision%29))
  (bind _returnvalue (Game|GetPlayerController 0))
  (bind (_locationx _locationy) (Game|Player|GetMousePosition _returnvalue))
  ;[1 1 1] 移动鼠标：【按住右键的同时移动鼠标】控制镜头旋转；【按住左键的同时移动鼠标】选择框
  (if (Variables|Default|Get是否触发框选)
    (bind _ashud_god (Utilities|Casting|CastToHUD_God (HUD|GetHUD _returnvalue)))
    (Variables|/Game/Games/Base/God/HUD_God.HUD_God_C|SetCurrent _ashud_god (Math|Vector2D|MakeVector2D _locationx _locationy))
    (elif (Variables|Default|Get是否可以转动屏幕)
      (Pawn|Input|AddControllerYawInput AxisValue))))

(fn ConstructionScript)

(fn 获得鼠标在地面的位置
  (bind _returnvalue (Game|GetPlayerController 0))
  (bind _hitresult (Game|Player|GetHitResultUnderCursorbyChannel _returnvalue "TraceTypeQuery1" true))
  (bind (_bblockinghit _binitialoverlap _time _distance _location _impactpoint _normal _impactnormal) (Collision|BreakHitResult _hitresult))
  (return _location (Math|Rotator|MakeRotationfromAxes _impactnormal "0, 0, 0" "0, 0, 0") _bblockinghit))

(fn 获得鼠标点击的棋子
  (bind _asbp_aibase (Utilities|Casting|CastToBP_AIBase (.HitActor (Collision|BreakHitResult (.HitResult (Game|Player|GetHitResultUnderCursorbyChannel (Game|GetPlayerController 0) "TraceTypeQuery3" true)))))
    (:then
      (return _asbp_aibase))
    (:CastFailed
      (return 0))))

(fn 清理上次选中的棋子的指示标
  (bind _被选中的棋子和脚底的指示标 (Variables|Default|Get被选中的棋子和脚底的指示标))
  (bind _keys (Utilities|Map|Keys _被选中的棋子和脚底的指示标))
  (for _array_element _keys
    (Utilities|IsValid (.Value (Utilities|Map|Find _被选中的棋子和脚底的指示标 _array_element))
      (:Is%20Valid
        (Actor|DestroyActor (.Value (Utilities|Map|Find _被选中的棋子和脚底的指示标 _array_element)))
        (Utilities|Map|Remove _被选中的棋子和脚底的指示标 _array_element)
        (if (== (Variables|/Game/Games/Base/AI/BP_AIBase.BP_AIBase_C|Get状态 _array_element) 0)
          (CallFunction|服务器：给棋子设定控制者 _array_element))))))

(fn 【线路】给选中的棋子设定目标
  (bind (_被点到的actor _是否找到) (控制|获得鼠标点击的能被追踪的Actor))
  (if _是否找到
    (bind _keys (Utilities|Map|Keys (Variables|Default|Get被选中的棋子和脚底的指示标)))
    (for _array_element _keys
      (Utilities|IsValid _array_element
        (:Is%20Valid
          (bind _是否 (控制|判断棋子是否有控制者 _array_element))
          (if _是否
            (Variables|/Game/Games/Base/AI/BP_AIBase.BP_AIBase_C|Set状态 _array_element 1)
            (bind _returnvalue (Utilities|Array|Add (Variables|/Game/Games/Base/AI/BP_AIBase.BP_AIBase_C|Get目标 _array_element) _被点到的actor))
            (Utilities|Array|SetArrayElem (Variables|/Game/Games/Base/AI/BP_AIBase.BP_AIBase_C|Get目标位置 _array_element) _returnvalue (Transformation|GetActorLocation _被点到的actor) true)
            (HUD|【移动/线路】更新HUD _array_element)
            (Utilities|Array|AddUnique (Variables|Default|Get【线路】已设定目标的棋子) _array_element)
            (CallFunction|服务器：给棋子设定控制者 _array_element self)))))
    (else
      (bind (_location _rotation _是否找到_2) (通用|获得鼠标在地面的位置))
      (if _是否找到_2
        (bind _keys_2 (Utilities|Map|Keys (Variables|Default|Get被选中的棋子和脚底的指示标)))
        (for _array_element_2 _keys_2
          (Utilities|IsValid _array_element_2
            (:Is%20Valid
              (bind _是否_2 (控制|判断棋子是否有控制者 _array_element_2))
              (if _是否_2
                (Variables|/Game/Games/Base/AI/BP_AIBase.BP_AIBase_C|Set状态 _array_element_2 1)
                (bind _returnvalue_2 (Utilities|Array|Add (Variables|/Game/Games/Base/AI/BP_AIBase.BP_AIBase_C|Get目标 _array_element_2) _array_element_2))
                (Utilities|Array|SetArrayElem (Variables|/Game/Games/Base/AI/BP_AIBase.BP_AIBase_C|Get目标位置 _array_element_2) _returnvalue_2 _location true)
                (HUD|【移动/线路】更新HUD _array_element_2)
                (Utilities|Array|AddUnique (Variables|Default|Get【线路】已设定目标的棋子) _array_element_2)
                (CallFunction|服务器：给棋子设定控制者 _array_element_2 self)))))))))

(fn 【线路】棋子开始沿着之前设定的目标走
  (for _array_element (Variables|Default|Get【线路】已设定目标的棋子)
    (Variables|/Game/Games/Base/AI/BP_AIBase.BP_AIBase_C|Set状态 _array_element 2)
    (CallFunction|【线路】服务器：棋子沿着目标走 _array_element (Utilities|Array|Get(acopy) (Variables|/Game/Games/Base/AI/BP_AIBase.BP_AIBase_C|Get目标 _array_element)) (Utilities|Array|Get(acopy) (Variables|/Game/Games/Base/AI/BP_AIBase.BP_AIBase_C|Get目标位置 _array_element)))))

(fn 【单次】让被选中的棋子立即执行一个目标
  (bind (_被点到的actor _是否找到) (控制|获得鼠标点击的能被追踪的Actor))
  (if _是否找到
    (bind _keys (Utilities|Map|Keys (Variables|Default|Get被选中的棋子和脚底的指示标)))
    (for _array_element _keys
      (Utilities|IsValid _array_element
        (:Is%20Valid
          (Utilities|Array|Clear (Variables|/Game/Games/Base/AI/BP_AIBase.BP_AIBase_C|Get目标 _array_element))
          (Utilities|Array|Clear (Variables|/Game/Games/Base/AI/BP_AIBase.BP_AIBase_C|Get目标位置 _array_element))
          (Utilities|Array|Add (Variables|/Game/Games/Base/AI/BP_AIBase.BP_AIBase_C|Get目标 _array_element) _被点到的actor)
          (Utilities|Array|Add :TargetArray (Variables|/Game/Games/Base/AI/BP_AIBase.BP_AIBase_C|Get目标位置 _array_element))
          (CallFunction|【单次】服务器：棋子移动到 _array_element (Transformation|GetActorLocation _被点到的actor))
          (Variables|/Game/Games/Base/AI/BP_AIBase.BP_AIBase_C|Set状态 _array_element 2)
          (HUD|【移动/线路】更新HUD _array_element)
          (CallFunction|服务器：给棋子设定控制者 _array_element self))))
    (else
      ;[1 1 1] 点击到地面
      (bind (_location _rotation _是否找到_2) (通用|获得鼠标在地面的位置))
      (if _是否找到_2
        (bind _keys_2 (Utilities|Map|Keys (Variables|Default|Get被选中的棋子和脚底的指示标)))
        (for _array_element_2 _keys_2
          (Utilities|IsValid _array_element_2
            (:Is%20Valid
              (bind _是否 (控制|判断棋子是否有控制者 _array_element_2))
              (if _是否
                (Utilities|Array|Clear (Variables|/Game/Games/Base/AI/BP_AIBase.BP_AIBase_C|Get目标 _array_element_2))
                (Utilities|Array|Clear (Variables|/Game/Games/Base/AI/BP_AIBase.BP_AIBase_C|Get目标位置 _array_element_2))
                (Utilities|Array|Add (Variables|/Game/Games/Base/AI/BP_AIBase.BP_AIBase_C|Get目标 _array_element_2) _array_element_2)
                (Utilities|Array|Add (Variables|/Game/Games/Base/AI/BP_AIBase.BP_AIBase_C|Get目标位置 _array_element_2) _location)
                (CallFunction|【单次】服务器：棋子移动到 _array_element_2 _location)
                (Variables|/Game/Games/Base/AI/BP_AIBase.BP_AIBase_C|Set状态 _array_element_2 2)
                (HUD|【移动/线路】更新HUD _array_element_2)
                (CallFunction|服务器：给棋子设定控制者 _array_element_2 self)))))))))

(fn 【单次/线路】棋子移动到一个目标后，更新棋子目标
  (params (棋子 :type BP%20AI%20Base%20Object%20Reference))
  (bind _目标 (Variables|/Game/Games/Base/AI/BP_AIBase.BP_AIBase_C|Get目标 棋子))
  (bind _目标位置 (Variables|/Game/Games/Base/AI/BP_AIBase.BP_AIBase_C|Get目标位置 棋子))
  (Utilities|Array|RemoveIndex _目标)
  (if (== (Utilities|Array|Length _目标) 0)
    (Utilities|Array|RemoveItem (Variables|Default|Get【线路】已设定目标的棋子) 棋子)
    (Variables|/Game/Games/Base/AI/BP_AIBase.BP_AIBase_C|Set状态 棋子 0)
    (Utilities|Array|Clear _目标位置)
    (HUD|【移动/线路】更新HUD 棋子)
    (if (not (Utilities|Map|Contains (Variables|Default|Get被选中的棋子和脚底的指示标) 棋子))
      (CallFunction|服务器：给棋子设定控制者 棋子))
    (else
      (Utilities|Array|RemoveIndex _目标位置)
      (CallFunction|【线路】服务器：棋子沿着目标走 棋子 (Utilities|Array|Get(acopy) _目标) (Utilities|Array|Get(acopy) _目标位置))
      (HUD|【移动/线路】更新HUD 棋子))))

(fn 【移动/线路】更新HUD
  (params (棋子 :type BP%20AI%20Base%20Object%20Reference))
  (bind _hud的目标位置 (LocalVariables|GetHUD的目标位置))
  (bind _ashud_god (Utilities|Casting|CastToHUD_God (HUD|GetHUD (Game|GetPlayerController 0))))
  (Utilities|IsValid 棋子
    (:Is%20Valid
      (bind _output_get (LocalVariables|Set当前棋子 棋子))
      (bind _output_get_2 (LocalVariables|SetHUD _ashud_god))
      (bind _array_element (Utilities|Array|ForEachLoopwithBreak (Variables|/Game/Games/Base/God/HUD_God.HUD_God_C|Get棋子的线结构体 _output_get_2) :!label _label)
        (:LoopBody
          (if (== (.所属棋子 (Utilities|Struct|BreakS_HUDPawnLine _array_element)) _output_get)
            (Utilities|Array|RemoveItem (Variables|/Game/Games/Base/God/HUD_God.HUD_God_C|Get棋子的线结构体 _output_get_2) _array_element)
            (goto _label Break)))
        (:Completed
          (Utilities|Array|Clear (LocalVariables|GetHUD的目标位置))
          (Utilities|IsValid _output_get
            (:Is%20Valid
              (LocalVariables|Set目标 (Variables|/Game/Games/Base/AI/BP_AIBase.BP_AIBase_C|Get目标 _output_get))
              (LocalVariables|Set目标位置 (Variables|/Game/Games/Base/AI/BP_AIBase.BP_AIBase_C|Get目标位置 _output_get))
              (Utilities|Array|Add (LocalVariables|GetHUD的目标位置) (Transformation|GetActorLocation (LocalVariables|Get当前棋子)))
              (for (_array_element_2 _array_index) (LocalVariables|Get目标)
                (if (== _array_element_2 (LocalVariables|Get当前棋子))
                  (Utilities|Array|Add _hud的目标位置 (Utilities|Array|Get(acopy) (LocalVariables|Get目标位置) _array_index))
                  (else
                    (Utilities|IsValid _array_element_2
                      (:Is%20Valid
                        (Utilities|Array|Add _hud的目标位置 (Transformation|GetActorLocation _array_element_2)))))))
              (Utilities|Array|Add (Variables|/Game/Games/Base/God/HUD_God.HUD_God_C|Get棋子的线结构体 (LocalVariables|GetHUD)) (Utilities|Struct|MakeS_HUDPawnLine (LocalVariables|Get当前棋子) (LocalVariables|GetHUD的目标位置))))))))))

(fn 判断棋子是否有控制者
  (params (棋子 :type BP%20AI%20Base%20Object%20Reference))
  (bind _self self)
  (bind _被选中的棋子和脚底的指示标 (Variables|Default|Get被选中的棋子和脚底的指示标))
  (bind _控制者 (Variables|/Game/Games/Base/AI/BP_AIBase.BP_AIBase_C|Get控制者 棋子))
  (bind _value (Utilities|Map|Find _被选中的棋子和脚底的指示标 棋子))
  (bind _returnvalue (== _控制者 0))
  (bind _returnvalue_2 (== _控制者 _self))
  (bind _returnvalue_3 (or _returnvalue _returnvalue_2))
  (Utilities|IsValid 棋子
    (:Is%20Valid
      (if _returnvalue_3
        (return _returnvalue_3)
        (else
          (Development|PrintString "有单位已经被其他玩家控制")
          (Utilities|IsValid _value
            (:Is%20Valid
              (Actor|DestroyActor _value)
              (Utilities|Map|Remove _被选中的棋子和脚底的指示标 棋子)
              (Utilities|Array|RemoveItem (Variables|Default|Get【线路】已设定目标的棋子) 棋子)
              (bind _ashud_god (Utilities|Casting|CastToHUD_God (HUD|GetHUD (Game|GetPlayerController 0))))
              (bind (_array_element _array_index) (Utilities|Array|ForEachLoopwithBreak (Variables|/Game/Games/Base/God/HUD_God.HUD_God_C|Get棋子的线结构体 _ashud_god) :!label _label)
                (:LoopBody
                  (if (== (.所属棋子 (Utilities|Struct|BreakS_HUDPawnLine _array_element)) 棋子)
                    (Utilities|Array|RemoveIndex (Variables|/Game/Games/Base/God/HUD_God.HUD_God_C|Get棋子的线结构体 _ashud_god) _array_index)
                    (goto _label Break)))
                (:Completed
                  (return _returnvalue_3))))))))))

(fn 选中棋子并在棋子底部生成指示标
  (params (棋子 :type BP%20AI%20Base%20Object%20Reference))
  (bind _是否 (控制|判断棋子是否有控制者 棋子))
  (if _是否
    (CallFunction|服务器：给棋子设定控制者 棋子 self)
    (bind _returnvalue (Game|SpawnActorfromClass "/Game/Games/Base/God/BP_Sign.BP_Sign_C" (Math|Conversions|ToTransform(Vector) (Transformation|GetWorldLocation (Variables|/Script/Engine.Character|GetMesh 棋子))) "AlwaysSpawn" 0 0))
    (Utilities|Map|Add (Variables|Default|Get被选中的棋子和脚底的指示标) 棋子 _returnvalue)
    (return)))

(fn 获得鼠标点击的能被追踪的Actor
  (bind _returnvalue (Game|GetPlayerController 0))
  (bind _hitresult (Game|Player|GetHitResultUnderCursorbyChannel _returnvalue "TraceTypeQuery4" true))
  (bind (_bblockinghit _binitialoverlap _time _distance _location _impactpoint _normal _impactnormal _physmat _hitactor) (Collision|BreakHitResult _hitresult))
  (return _hitactor _bblockinghit))

(fn 摧毁棋子
  (params (棋子 :type BP%20AI%20Base%20Object%20Reference))
  (bind _被选中的棋子和脚底的指示标 (Variables|Default|Get被选中的棋子和脚底的指示标))
  (Actor|DestroyActor (.Value (Utilities|Map|Find _被选中的棋子和脚底的指示标 棋子)))
  (Utilities|Map|Remove _被选中的棋子和脚底的指示标 棋子)
  (Utilities|Array|RemoveItem (Variables|Default|Get【线路】已设定目标的棋子) 棋子)
  (CallFunction|服务器：摧毁棋子 棋子))