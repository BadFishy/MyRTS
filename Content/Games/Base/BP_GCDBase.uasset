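; BP_GCDBase is a base playable-character Blueprint handling movement, camera, rotation, mouse-cursor toggling and animation emotes.
; BeginPlay loads animations and playback modes from the data table row matching its class name, then builds an action-list widget in PC_GCD's main bar.
; Inputs toggle that list or use quick-bar items by key.
; Server-labelled events pass the movement axis and set the playing animation name and flag by index.
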(event Collision|EventActorBeginOverlap
  (params (OtherActor :type Actor%20Object%20Reference)))

(event EventTick
  (params (DeltaSeconds :type Float%20%28single-precision%29)))

(event Custom|生成角色动作列表Bar
  ;[1 1 1] 初始化：生成角色动作列表Bar
  (bind _returnvalue (UserInterface|CreateWidget "/Game/Games/Base/Bar/AnimationBox/W_AnimationBox.W_AnimationBox_C" (Game|GetPlayerController 0) (Variables|Default|GetAnimation) (Variables|Default|GetAnimationState) (Variables|Default|GetBar主控件) "动作列表[O]"))
  (bind _output_get (Variables|Default|Set动作列表Bar控件 _returnvalue))
  (Widget|Panel|AddChild (Variables|/Game/Games/Base/Bar/W_BarMain.W_BarMain_C|Get右侧Bar (Variables|Default|GetBar主控件)) _output_get))

(event EventBeginPlay
  ;[1 1 1] 初始化：从数据表中获得可用动作
  (Utilities|FlowControl|Sequence
    (:then_0
      (bind _returnvalue (Utilities|GetDataTableRow (Variables|Default|Get角色数据表) (Utilities|String|StringToName (Utilities|String|Replace (Utilities|GetClassDisplayName (Utilities|GetClass self)) "_C")))
        (:then
          (Variables|Default|SetAnimation (.AnimSequence (Utilities|Struct|BreakS_Actor _returnvalue)))
          (Variables|Default|SetAnimationState (.AnimSequenceName是播放一次0是循环1还是结束后保持最后状态2 (Utilities|Struct|BreakS_Actor _returnvalue))))
        (:RowNotFound
          (Development|PrintString "没有找到这个Actor的数据表行"))))
    (:then_1
      ;[1 1 1] 生成Bar
      (bind _aspc_gcd (Utilities|Casting|CastToPC_GCD (Game|GetPlayerController 0)))
      (Variables|Default|SetBar主控件 (Variables|/Game/Games/Base/PC_GCD.PC_GCD_C|GetBar主控件 _aspc_gcd))
      (Variables|Default|Set底部快捷栏Bar控件 (Variables|/Game/Games/Base/PC_GCD.PC_GCD_C|Get底部快捷栏Bar控件 _aspc_gcd))
      (CallFunction|生成角色动作列表Bar))))

(event Custom|服务器获得Axis
  (params (Axis :type Vector%202D%20Structure))
  ;[1 1 1] 键盘控制旋转
  (Variables|Default|SetAxis Axis))

(event Custom|呼出/隐藏鼠标
  (bind _returnvalue (Game|GetPlayerController 0))
  (bind (_sizex _sizey) (HUD|GetViewportSize _returnvalue))
  ;[1 1 1] 呼出/隐藏鼠标
  (Utilities|FlowControl|FlipFlop
    (:A
      (Input|SetInputModeGameandUI _returnvalue (Variables|Default|GetBar主控件) "DoNotLock" true)
      (Class|PlayerController|SetMouseLocation _returnvalue (/ _sizex 2) (/ _sizey 2))
      (Variables|/Script/Engine.PlayerController|SetbShowMouseCursor _returnvalue true))
    (:B
      (Input|SetInputModeGameOnly _returnvalue)
      (Variables|/Script/Engine.PlayerController|SetbShowMouseCursor _returnvalue false))))

(event Input|ActionEvents|InputAction通用：数字快捷栏（顺序不能错）
  (params (Key :type Key%20Structure))
  ;[1 1 1] 数字键：使用快捷栏的道具
  (:Pressed
    (bind _asw_bar_item_base (Utilities|Casting|CastToW_BarItemBase (Class|PanelWidget|GetChildat (Variables|/Game/Games/Base/Bar/Base/W_BarSlot.W_BarSlot_C|Get项目ItemBase (.Value (Utilities|Map|Find (Variables|/Game/Games/Base/Bar/ShortcutBar/W_ShortcutBar.W_ShortcutBar_C|Get按键-格子 (Variables|Default|Get底部快捷栏Bar控件)) Key))))))
    (Default|使用 _asw_bar_item_base)))

(event Input|ActionEvents|InputAction角色模式：呼出动作列表
  (params (Key :type Key%20Structure))
  ;[1 1 1] 打开动作菜单UI
  (:Pressed
    (Default|显示/隐藏Bar (Variables|Default|GetBar主控件) (Variables|Default|Get动作列表Bar控件))))

(event Input|ActionEvents|InputAction角色模式：呼出鼠标
  (params (Key :type Key%20Structure))
  ;[1 1 1] 呼出/隐藏鼠标
  (:Pressed
    (CallFunction|呼出/隐藏鼠标)))

(event Input|AxisEvents|InputAxis角色模式：旋转角色
  (params (AxisValue :type Float%20%28single-precision%29))
  ;[1 1 1] 键盘控制旋转
  (Class|Actor|AddActorWorldRotation (Math|Rotator|MakeRotator 0.0 0.0 (* 6 AxisValue))))

(event Input|AxisEvents|InputAxis通用：纵向移动
  (params (AxisValue :type Float%20%28single-precision%29))
  (bind _returnvalue (Pawn|GetControlRotation :!class /Script/Engine.Pawn))
  (bind _yaw (Math|Rotator|BreakRotator _returnvalue))
  (bind _returnvalue_2 (Math|Rotator|MakeRotator 0.0 0.0 _yaw))
  ;[1 1 1] WASD控制
  (Variables|Default|SetAxis (Math|Vector2D|MakeVector2D (.x (Variables|Default|GetAxis)) AxisValue))
  ;;[1 1 1] 移动
  (CallFunction|服务器获得Axis (Variables|Default|GetAxis))
  (Pawn|Input|AddMovementInput (+ (* (Math|Vector|GetForwardVector _returnvalue_2) (.y (Variables|Default|GetAxis))) (* (Math|Vector|GetRightVector _returnvalue_2) (.x (Variables|Default|GetAxis)))) 1.0 false))

(event Input|AxisEvents|InputAxis通用：横向移动
  (params (AxisValue :type Float%20%28single-precision%29))
  (bind _returnvalue (Pawn|GetControlRotation :!class /Script/Engine.Pawn))
  (bind _yaw (Math|Rotator|BreakRotator _returnvalue))
  (bind _returnvalue_2 (Math|Rotator|MakeRotator 0.0 0.0 _yaw))
  ;[1 1 1] WASD控制
  (Variables|Default|SetAxis (Math|Vector2D|MakeVector2D AxisValue (.y (Variables|Default|GetAxis))))
  ;;[1 1 1] 移动
  (CallFunction|服务器获得Axis (Variables|Default|GetAxis))
  (Pawn|Input|AddMovementInput (+ (* (Math|Vector|GetForwardVector _returnvalue_2) (.y (Variables|Default|GetAxis))) (* (Math|Vector|GetRightVector _returnvalue_2) (.x (Variables|Default|GetAxis)))) 1.0 false))

(event Input|AxisEvents|InputAxis通用：上下看
  (params (AxisValue :type Float%20%28single-precision%29))
  ;[1 1 1] 鼠标控制镜头旋转
  (Pawn|Input|AddControllerPitchInput AxisValue))

(event Input|AxisEvents|InputAxis通用：左右看
  (params (AxisValue :type Float%20%28single-precision%29))
  ;[1 1 1] 鼠标控制镜头旋转
  (Pawn|Input|AddControllerYawInput AxisValue))

(event Custom|弹起动作表情
  ;[1 1 1] 服务器：播放动作表情
  (Variables|Default|SetIsPlayingAnim false))

(event Custom|按下动作表情
  (params (NewParam :type Integer))
  ;[1 1 1] 服务器：播放动作表情
  (bind _keys (Utilities|Map|Keys (Variables|Default|GetAnimation)))
  (Variables|Default|SetPlayingAnimName (Utilities|Array|Get(acopy) _keys NewParam))
  (Variables|Default|SetIsPlayingAnim true))

(event Custom|动作表情
  (params (NewParam :type Integer))
  ;[1 1 1] 服务器：播放动作表情
  (CallFunction|按下动作表情 NewParam)
  (bind _keys (Utilities|Map|Keys (Variables|Default|GetAnimation)))
  (Variables|Default|SetPlayingAnimName (Utilities|Array|Get(acopy) _keys (stale Custom|按下动作表情 NewParam)))
  (Variables|Default|SetIsPlayingAnim true))

(fn ConstructionScript)