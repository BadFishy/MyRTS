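; AI base Blueprint for a piece (棋子) that follows a queued route of targets managed by its controller (控制者).
; In state 2, Tick refreshes later actor targets' positions for the route HUD, while a valid first target is re-inserted at the front and reported to the controller.
; Invalid targets are removed and movement resumes.
; Self entries act as location waypoints, reporting arrival once when the piece stops near the first position.
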(event EventTick
  (params (DeltaSeconds :type Float%20%28single-precision%29))
  (bind _目标位置 (Variables|Default|Get目标位置))
  (bind _目标位置_2 (Variables|Default|Get目标位置))
  (bind _控制者 (Variables|Default|Get控制者))
  (bind _控制者_2 (Variables|Default|Get控制者))
  (bind _目标 (Variables|Default|Get目标))
  (bind _output (Utilities|Array|Get(acopy) _目标位置_2))
  (if (== (Variables|Default|Get状态) 2)
    (for (_array_element _array_index) (Variables|Default|Get目标)
      (if (!= _array_element self)
        (Utilities|IsValid _array_element
          (:Is%20Valid
            (if (== _array_index 0)
              (Utilities|Array|Insert _目标 (Utilities|Array|Get(acopy) _目标 _array_index))
              (Utilities|Array|Insert (Variables|Default|Get目标位置) (Transformation|GetActorLocation (Utilities|Array|Get(acopy) _目标 _array_index)))
              (Default|【单次/线路】棋子移动到一个目标后，更新棋子目标 _控制者_2 self)
              (else
                (Utilities|Array|SetArrayElem _目标位置 _array_index (Transformation|GetActorLocation _array_element) true)
                (Default|【移动/线路】更新HUD _控制者_2 self :!label _label))))
          (:Is%20Not%20Valid
            (Utilities|Array|RemoveIndex _目标 _array_index)
            (Utilities|Array|RemoveIndex _目标位置 _array_index)
            (Default|【线路】棋子开始沿着之前设定的目标走 _控制者)
            (goto _label)))
        (else
          ;[1 1 1] 判断棋子是否已经移动到目标
          (if (Math|Vector|Equal(Vector) (Transformation|GetWorldLocation (Variables|Character|GetMesh)) _output 5e+01)
            (if (not (or (Math|Vector|Equal(Vector) _output (Variables|Default|Get上次目标) 0.0) (> (Math|Vector|VectorLength (Transformation|GetVelocity)) 1.0)))
              (Variables|Default|Set上次目标 _output)
              (Utilities|IsValid _控制者
                (:Is%20Valid
                  (Default|【单次/线路】棋子移动到一个目标后，更新棋子目标 _控制者 self))))))))))

(fn ConstructionScript)